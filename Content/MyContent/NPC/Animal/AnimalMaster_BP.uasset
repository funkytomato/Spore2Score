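; AnimalMaster_BP is an NPC animal that grazes, defecates, sleeps and dies.
; A looping timer drains Health through LifeCycle, calling OnDeath at zero to stop tick and unpossess.
; FeedProximity overlaps flag nearby growables and the player, while Grazing restores Health and, when high enough, flags defecation, which spawns Poo_BP.
; RunAway is empty, and the GettingTired timer is disconnected.
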(event `self.ReceiveBeginPlay`
  ;[1 1 1] Beginplay - Set the timer for becoming Tired and the Animal LifeCycle
  (`KismetSystemLibrary.K2_SetTimer` null "LifeCycle" 1.0 true))

(event `GettingTired`
  ;[1 1 1] Beginplay - Set the timer for becoming Tired and the Animal LifeCycle
  (set `self.IsTired` true))

(event `self.FeedProximity.OnComponentBeginOverlap`
  (params (OverlappedComponent :type "PrimitiveComponent Object Reference") (OtherActor :type "Actor Object Reference") (OtherComp :type "PrimitiveComponent Object Reference") (OtherBodyIndex :type Integer) (bFromSweep :type Boolean) (SweepResult :type "HitResult Structure (by ref)"))
  ;[1 1 1] Can graze if near Growables (grass)
  (bind _asgrowable_master_bp (cast `/Game/MyContent/Growable/GrowableMaster_BP` OtherActor)
    (:`then`
      (set `self.CanGraze` true))
    (:`CastFailed`
      (cast `/Game/MyContent/Characters/Blueprints/Spore2ScoreCharacter` OtherActor)
      (set `self.PlayerNearby` true))))

(event `self.FeedProximity.OnComponentEndOverlap`
  (params (OverlappedComponent :type "PrimitiveComponent Object Reference") (OtherActor :type "Actor Object Reference") (OtherComp :type "PrimitiveComponent Object Reference") (OtherBodyIndex :type Integer))
  ;[1 1 1] Can graze if near Growables (grass)
  (cast `/Game/MyContent/Growable/GrowableMaster_BP` OtherActor
    (:`then`
      (set `self.CanGraze` false))
    (:`CastFailed`
      (cast `/Game/MyContent/Characters/Blueprints/Spore2ScoreCharacter` OtherActor)
      (set `self.PlayerNearby` false))))

(event `/Game/MyContent/NPC/Animal/Animal_BPI.Grazing`
  ;[1 1 1] Grazing increases health of the animal and makes it want to defecate
  (`KismetSystemLibrary.PrintString` "Animal is grazing")
  (set `self.IsGrazing` true)
  (set `self.HasDefecated` false)
  (set `self.Health` (`KismetMathLibrary.FClamp` (+ (`self.Health`) 5.0) 0.0 100.0))
  (if (>= (`self.Health`) 80.0)
    (set `self.NeedsToDefecate` true)
    (`KismetSystemLibrary.Delay` 2.0)
    (set `self.IsGrazing` false)
    (set `self.CanGraze` false)))

(event `/Game/MyContent/NPC/Animal/Animal_BPI.Defecating`
  ;[1 1 1] Defecated
  (`/Engine/EditorBlueprintResources/StandardMacros.DoOnce` false :!label _label
    (:`Completed`
      (`|SpawnActorFromClass` "/Game/MyContent/NPC/Poo/Poo_BP.Poo_BP_C" (`SceneComponent.K2_GetComponentToWorld` (`self.PooExit`)) "Undefined" "OverrideRootScale" null self)
      (`KismetSystemLibrary.Delay` 2.0)
      (set `self.NeedsToDefecate` false)
      (set `self.HasDefecated` true)
      (goto _label :!via `Reset`))))

(event `/Game/MyContent/NPC/Animal/Animal_BPI.RunAway`
  (params (LocationToRunawayFrom :type "Vector Structure"))
  ;[1 1 1] Run away from location
)

(event `/Game/MyContent/NPC/Animal/Animal_BPI.Sleeping`
  ;[1 1 1] Sleep
  (set `self.IsSleeping` true)
  (`KismetSystemLibrary.Delay` (`self.SleepLength`))
  (set `self.IsTired` false)
  (set `self.IsSleeping` false))

(event `OnDeath`
  ;[1 1 1] OnDeath
  (`self.SetActorTickEnabled` false)
  (`Controller.UnPossess` (`self.GetController`))
  (set `self.IsDead` true))

(fn `LifeCycle`
  ;[1 1 1] Reduce health each cycle
  (set `self.Health` (`KismetMathLibrary.FClamp` (- (`self.Health`) 0.1) 0.0 100.0))
  ;[1 1 1] Am I alive?
  (if (<= (`self.Health`) 0.0)
    (`self.OnDeath`)))

(fn `UserConstructionScript`)