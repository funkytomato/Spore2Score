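; AnimalOld_BP is an NPC animal that tracks grazing, tiredness, defecation and death through state flags.
; Looping timers mark it tired every minute and poll Health each second in LifeCycle to flag death.
; FeedProximity overlaps flag whether it can graze on sufficiently healthy GrowableMaster_BP plants and whether a Spore2ScoreCharacter is nearby.
; The IsGrazing event raises Health and flags the need to defecate once full, which IsDefectating clears.
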(event `self.ReceiveBeginPlay`
  ;[1 1 1] Beginplay - Set the timer for becoming Tired and the Animal LifeCycle
  (`KismetSystemLibrary.K2_SetTimerDelegate` (delegate `GettingTired`) 60.0 true)
  (`KismetSystemLibrary.K2_SetTimer` null "LifeCycle" 1.0 true))

(event `GettingTired`
  ;[1 1 1] Beginplay - Set the timer for becoming Tired and the Animal LifeCycle
  (set `self.IsTired` true))

(event `self.FeedProximity.OnComponentBeginOverlap`
  (params (OverlappedComponent :type "PrimitiveComponent Object Reference") (OtherActor :type "Actor Object Reference") (OtherComp :type "PrimitiveComponent Object Reference") (OtherBodyIndex :type Integer) (bFromSweep :type Boolean) (SweepResult :type "HitResult Structure (by ref)"))
  ;[1 1 1] Can graze if near Growables (grass)
  (bind _asgrowable_master_bp (cast `/Game/MyContent/Growable/GrowableMaster_BP` OtherActor)
    (:`then`
      (if (>= (`/Game/MyContent/Growable/GrowableMaster_BP.Health` _asgrowable_master_bp) 80.0)
        (set `self.CanGraze` true)))
    (:`CastFailed`
      (cast `/Game/MyContent/Characters/Blueprints/Spore2ScoreCharacter` OtherActor)
      (set `self.PlayerNearby` true))))

(event `self.FeedProximity.OnComponentEndOverlap`
  (params (OverlappedComponent :type "PrimitiveComponent Object Reference") (OtherActor :type "Actor Object Reference") (OtherComp :type "PrimitiveComponent Object Reference") (OtherBodyIndex :type Integer))
  ;[1 1 1] Can graze if near Growables (grass)
  (cast `/Game/MyContent/Growable/GrowableMaster_BP` OtherActor
    (:`then`
      (set `self.CanGraze` false))
    (:`CastFailed`
      (cast `/Game/MyContent/Characters/Blueprints/Spore2ScoreCharacter` OtherActor)
      (set `self.PlayerNearby` false))))

(event `IsGrazing`
  ;[1 1 1] Grazing increases health of the animal and makes it want to defecate
  (set `self.Health` (+ (`self.Health`) 5.0))
  (if (>= (`self.Health`) 100.0)
    (set `self.NeedsToDefecate` true)))

(event `IsDefectating`
  ;[1 1 1] Defecated
  (set `self.NeedsToDefecate` false)
  (set `self.HasDefecated` true))

(fn `LifeCycle`
  (if (<= (`self.Health`) 0.0)
    (set `self.IsDead` true)))

(fn `UserConstructionScript`)