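; GrowableMaster_BP is a growable object, apparently a base class by its name, whose static mesh shows or hides based on a Health value.
; BeginPlay binds an IncreaseHealth event that adds clamped health and starts a looping one-second timer on LifeCycle.
; LifeCycle toggles mesh visibility at a health threshold.
; A DecreaseHealth decay function exists, but its call in LifeCycle is disconnected, so health never drops here.
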(event `self.ReceiveBeginPlay`
  (add `self.Increase Health` (delegate `Increase Health_Event`))
  (`KismetSystemLibrary.K2_SetTimer` null "LifeCycle" 1.0 true))

(event `Increase Health_Event`
  (set `self.Health` (`KismetMathLibrary.FClamp` (+ (`self.Health`) 10.0) 0.0 100.0)))

(fn `DecreaseHealth`
  (set `self.Health` (`KismetMathLibrary.FClamp` (- (`self.Health`) 1.0) 0.0 100.0)))

(fn `LifeCycle`
  (bind _staticmesh (`self.StaticMesh`))
  (if (>= (`self.Health`) 20.0)
    (`SceneComponent.SetVisibility` _staticmesh true false)
    (else
      (`SceneComponent.SetVisibility` _staticmesh false false))))

(fn `UserConstructionScript`)