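; BiologicalMaster_BP is a base Blueprint for plant-like interactable items that exchange nutrients with a Mysellium network.
; A looping timer runs the health cycle, sending nutrients to the Mysellium when connected and draining health otherwise.
; At full health, connected plants boost and mark as connected nearby Growables, cached once from a sphere overlap shortly after BeginPlay.
; Low health flags the plant unhealthy and reduces its nutrient amount, which also sets the drain rate.
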(event `self.ReceiveBeginPlay`
  (`parent.ReceiveBeginPlay`)
  (`KismetSystemLibrary.Delay` 1.0)
  (set `self.Growables` (`PrimitiveComponent.GetOverlappingActors` (`self.MyselliumSphereOfInfluence`) "/Game/MyContent/Environment/SpawnedGrowables/GrowableMaster_BP.GrowableMaster_BP_C"))
  (`KismetSystemLibrary.K2_SetTimer` null "Plant Health Cycle" 1.0 true))

(fn `IncreaseGrassHealthWithinProximity`
  (for _array_element (`self.Growables`)
    (bind _asgrowable_master_bp (cast `/Game/MyContent/Environment/SpawnedGrowables/GrowableMaster_BP` _array_element)
      (:`then`
        (`/Game/MyContent/Environment/SpawnedGrowables/GrowableMaster_BP.Increase Health` _asgrowable_master_bp)
        (set `/Game/MyContent/Environment/SpawnedGrowables/GrowableMaster_BP.MyselliumConnected` true _asgrowable_master_bp))
      (:`CastFailed`
        (`KismetSystemLibrary.PrintString` "BiologicalMaster - Failed to cast GrowableMaster")))))

(fn `Plant Health Cycle`
  ;[1 1 1] Plant shall lose health over time, but could send it too Mysellium
  (if (`self.ConnectedToMyselliumTrail`)
    (`/Game/MyContent/Environment/Mysellium/Mysellium_BP.Recieve Nutrients` (`self.Mysellium_Ref`) (`self.NutrientAmountToSend`))
    (if (>= (`self.Health`) 100.0)
      (`self.IncreaseGrassHealthWithinProximity`))
    (else
      (bind _output_get (set `self.Health` (`KismetMathLibrary.FClamp` (- (`self.Health`) (`self.NutrientAmountToSend`)) 0.0 (`self.MaxHealth`))))))
  ;[1 1 1] Set Unhealthy flag if sick
  (if (< _output_get (`self.LowHealthValue`))
    (set `self.IsUnhealthy` true)
    (set `self.NutrientAmountToSend` 1.0)
    (else
      (set `self.IsUnhealthy` false)
      (set `self.NutrientAmountToSend` 5.0))))

(fn `UserConstructionScript`
  (`parent.UserConstructionScript`))