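; Master Blueprint for leafy trees whose appearance reflects their health.
; A looping one-second timer hides the leaves at or below the low-health threshold and shows them otherwise.
; At full health, each timer pass also slightly increases the world scale of the tree mesh and leaves, with no upper limit.
; GrowLeaves and LeavesFall are called on every corresponding pass but are empty here.
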(event `self.ReceiveBeginPlay`
  (`parent.ReceiveBeginPlay`)
  (`KismetSystemLibrary.K2_SetTimer` null "Update Visual Representation to Health" 1.0 true))

(fn `Grow`
  (bind _staticmesh (`self.StaticMesh`))
  (`SceneComponent.SetWorldScale3D` _staticmesh (+ (`SceneComponent.K2_GetComponentScale` _staticmesh) 0.001))
  (`SceneComponent.SetWorldScale3D` (`self.Leaves`) (+ (`SceneComponent.K2_GetComponentScale` (`self.Leaves`)) 0.001)))

(fn `GrowLeaves`)

(fn `LeavesFall`)

(fn `Update Visual Representation to Health`
  (bind _leaves (`self.Leaves`))
  ;[1 1 1] Show/Not Show Leaves according to health
  (if (<= (`self.Health`) (`self.LowHealthValue`))
    (`SceneComponent.SetVisibility` _leaves false false)
    (`self.LeavesFall`)
    (else
      (`SceneComponent.SetVisibility` _leaves true false)
      (`self.GrowLeaves`)
      (if (>= (`self.Health`) 100.0)
        (`self.Grow`)))))

(fn `UserConstructionScript`
  (`parent.UserConstructionScript`))