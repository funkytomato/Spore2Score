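; Base Blueprint for interactable environment items such as plants and rocks, tracking health, nutrients and pollution.
; Nutrient events from Mysellium_BP feed nutrients, which raise health when high, while depletion lowers it.
; Player overlap toggles a health widget, turned toward the follow camera once on entry, and refreshes the health visual, which currently only hides the light.
; Interact branches on polluted, breakable or huggable flags but only prints placeholder messages.
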(event `RotateToFacePlayer`
  ;[1 1 1] Rotate Widget to face Player
  (bind _asspore_2score_character (cast `/Game/MyContent/Characters/Blueprints/Spore2ScoreCharacter` (`GameplayStatics.GetPlayerCharacter` 0)))
  (`SceneComponent.K2_SetWorldRotation` (`self.Widget`) (`KismetMathLibrary.FindLookAtRotation` (`SceneComponent.K2_GetComponentLocation` (`self.DefaultSceneRoot`)) (`SceneComponent.K2_GetComponentLocation` (`/Game/MyContent/Characters/Blueprints/Spore2ScoreCharacter.FollowCamera` _asspore_2score_character))) false false))

(event `IncreaseHealth`
  (params (HealthAmount :type "Float (double-precision)"))
  ;[1 1 1] Update Health Property
  (set `self.Health` (`KismetMathLibrary.FClamp` (+ HealthAmount (`self.Health`)) 0.0 (`self.MaxHealth`))))

(event `ReducePollution`
  (params (AmountToReduce :type "Float (double-precision)"))
  ;[1 1 1] Update Pollution Level
  (set `self.PollutionLevel` (- AmountToReduce (`self.PollutionLevel`))))

(event `IncreaseNutrients`
  (params (amount :type "Float (double-precision)"))
  ;[1 1 1] Update Nutrients Property
  (set `self.Nutrients` (`KismetMathLibrary.FClamp` (+ amount (`self.Nutrients`)) 0.0 (`self.MaxNutrients`)))
  (if (>= (`self.Nutrients`) 100.0)
    (`self.IncreaseHealth` 5.0)))

(event `IncreasePollution`
  (params (AmountToIncrease :type "Float (double-precision)"))
  ;[1 1 1] Update Pollution Level
  (set `self.PollutionLevel` (+ AmountToIncrease (`self.PollutionLevel`))))

(event `DecreaseNutrients`
  (params (amount :type "Float (double-precision)"))
  ;[1 1 1] Update Nutrients Property
  (set `self.Nutrients` (`KismetMathLibrary.FClamp` (- (`self.Nutrients`) amount) 0.0 (`self.MaxNutrients`)))
  (if (<= (`self.Nutrients`) 0.0)
    (`self.DecreaseHealth` amount)))

(event `DecreaseHealth`
  (params (DecreaseAmount :type "Float (double-precision)"))
  ;[1 1 1] Update Health Property
  (set `self.Health` (`KismetMathLibrary.FClamp` (- (`self.Health`) DecreaseAmount) 0.0 (`self.MaxHealth`))))

(event `self.InteractionSphereOfInfluence.OnComponentBeginOverlap`
  (params (OverlappedComponent :type "PrimitiveComponent Object Reference") (OtherActor :type "Actor Object Reference") (OtherComp :type "PrimitiveComponent Object Reference") (OtherBodyIndex :type Integer) (bFromSweep :type Boolean) (SweepResult :type "HitResult Structure (by ref)"))
  ;[1 1 1] Update Plant Illumination/Sparkle corresponding plant Health and show the Health widget
  (cast `/Game/MyContent/Characters/Blueprints/Spore2ScoreCharacter` OtherActor)
  (`self.Update Plant Health Visual`)
  (`self.RotateToFacePlayer`)
  (`SceneComponent.SetVisibility` (`self.Widget`) true false))

(event `/Game/MyContent/Interface/Score2Spore_BPI.Interact`
  ;[1 1 1] Interact with Game Items
  ;;[1 1 1] Cleanup Pollution
  (if (`self.Polluted`)
    (`KismetSystemLibrary.PrintString` "Clean Pollution")
    (else
      ;;[1 1 1] Is a rock, smash it, to release minerals
      (if (`self.Breakable`)
        (`KismetSystemLibrary.PrintString` "Smash Rock")
        (else
          ;;[1 1 1] Hug Tree, give some love
          (if (`self.Huggable`)
            (`KismetSystemLibrary.PrintString` "Hug!!!")))))))

(event `self.InteractionSphereOfInfluence.OnComponentEndOverlap`
  (params (OverlappedComponent :type "PrimitiveComponent Object Reference") (OtherActor :type "Actor Object Reference") (OtherComp :type "PrimitiveComponent Object Reference") (OtherBodyIndex :type Integer))
  ;[1 1 1] Update Plant Illumination/Sparkle corresponding plant Health and show the Health widget
  (cast `/Game/MyContent/Characters/Blueprints/Spore2ScoreCharacter` OtherActor)
  (`self.Update Plant Health Visual`)
  (`SceneComponent.SetVisibility` (`self.Widget`) false false))

(event `self.ReceiveBeginPlay`
  ;[1 1 1] Get reference to Mysellium BP
  (bind _returnvalue (`GameplayStatics.GetActorOfClass` "/Game/MyContent/Environment/Mysellium/Mysellium_BP.Mysellium_BP_C"))
  (set `self.Mysellium_Ref` _returnvalue)
  ;[1 1 1] Get Reference to Widget_BP
  (bind _asbio_widget_bp (cast `/Game/MyContent/Widgets/BioWidget_BP` (`WidgetComponent.GetUserWidgetObject` (`self.Widget`))))
  (bind _output_get (set `self.HealthWidget` _asbio_widget_bp))
  (set `/Game/MyContent/Widgets/BioWidget_BP.OwningActor` self _output_get)
  ;[1 1 1] Show the Plant's Health status on BeginPlay
  (`self.Update Plant Health Visual`)
  ;[1 1 1] Boost Health from Mysellium
  (add `self.ReceiveNutrients` (delegate `ReceiveNutrients_Event`)))

(event `ReceiveNutrients_Event` :!signature `self.ReceiveNutrients`
  (params (Amount :type "Float (double-precision)"))
  ;[1 1 1] Boost Health from Mysellium
  (`self.IncreaseNutrients` Amount)
  (set `self.RecievedNutrientAmount` Amount))

(fn `Illuminate`
  (params (IsOn :type Boolean))
  (bind _illuminationlight (`self.IlluminationLight`))
  (if IsOn
    (`SceneComponent.SetVisibility` _illuminationlight true false)
    (else
      (`SceneComponent.SetVisibility` _illuminationlight false false))))

(fn `IsHealthy`
  (returns (IsHealthy :type Boolean))
  (return (>= (`self.Health`) (`self.LowHealthValue`))))

(fn `IsMaxHealth`
  (returns (FullHealth :type Boolean))
  (return (>= (`self.Health`) 100.0)))

(fn `IsPolluted`
  (returns (IsPolluted :type Boolean))
  (bind _returnvalue (>= (`self.PollutionLevel`) (`self.HighPollutionValue`)))
  (if _returnvalue
    (set `self.Polluted` true)
    (else
      (set `self.Polluted` false)))
  (return _returnvalue))

(fn `MyselliumBonus`
  (if (`self.ConnectedToMyselliumTrail`)
    (set `self.Health` (`KismetMathLibrary.FClamp` (+ (`self.Health`) (`self.MySelliumHealthBonus`)) 0.0 100.0))))

(fn `ShowPollution`
  (bind _pollutiondecal (`self.PollutionDecal`))
  (if (`self.Polluted`)
    (`SceneComponent.SetVisibility` _pollutiondecal true false)
    (else
      (`SceneComponent.SetVisibility` _pollutiondecal false false))))

(fn `Sparkle`
  (`KismetSystemLibrary.PrintString` "Make Tree Sparkle")
  (`ActorComponent.SetActive` (`self.SparkleParticles`) false false))

(fn `UnIlluminate`
  (`SceneComponent.SetVisibility` (`self.IlluminationLight`) false false))

(fn `Update Plant Health Visual`
  ;[1 1 1] Make Plant Sparkle if healthy
  (bind _ishealthy (`self.IsHealthy`))
  (if _ishealthy
    (`self.UnIlluminate`)
    (else
      (`self.Illuminate` false))))

(fn `UpdateHealth`
  (set `self.Health` (- (`self.HealthLoss`) (`self.Health`)))
  (`self.MyselliumBonus`))

(fn `UserConstructionScript`)