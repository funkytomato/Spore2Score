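; Mysellium actor that acts as the level's nutrient network, tracking connected lifeforms, its own health and win or fail state.
; Bound events add or remove life and receive nutrients.
; A looping timer checks level outcome, then distributes nutrients by each member's condition, draining health when supply runs low.
; Illumination events toggle glow on connected life while switching the directional light off or on to highlight the trail.
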(event `AddWidget`
  ;[1 1 1] BeginPlay - Get reference to Widget_BP
  (bind _asmysellium_widget_bp (cast `/Game/MyContent/Widgets/MyselliumWidget_BP` (`WidgetComponent.GetUserWidgetObject` (`self.Widget`))))
  (bind _output_get (set `self.MyselliumWidget` _asmysellium_widget_bp))
  (set `/Game/MyContent/Widgets/MyselliumWidget_BP.OwningActor` self _output_get))

(event `CheckLevelSuccess`
  ;[1 1 1] Show Level Complete Menu
  (if (> (`KismetArrayLibrary.Array_Length` (`self.MyselliumLife`)) (`self.LifeformWinCount`))
    (if (>= (`self.Nutrients`) 100.0)
      (bind _asspore_2score_game_instance (cast `/Game/MyContent/Blueprints/Spore2ScoreGameInstance` (`GameplayStatics.GetGameInstance`)))
      (`/Game/MyContent/Blueprints/Spore2ScoreGameInstance.ShowLevelCompleteMenu` _asspore_2score_game_instance))))

(event `self.ReceiveBeginPlay`
  ;[1 1 1] Initialise and configure Messages
  (add `self.Add Life To Mysellium` (delegate `AddLifeToMysellium_Event`))
  (add `self.Remove Life From Mysellium` (delegate `Remove Life From Mysellium_Event`))
  (add `self.Recieve Nutrients` (delegate `Recieve Nutrients_Event`))
  ;[1 1 1] Mysellium Life Cycle
  (`KismetSystemLibrary.K2_SetTimerDelegate` (delegate `MyselliumLifeCycleTick`) 1.0 true))

(event `MyselliumLifeCycleTick`
  ;[1 1 1] Mysellium Life Cycle
  (`self.CheckLevelSuccess`)
  (`self.CheckLevelFailed`)
  (`self.Send Nutrients to Life`))

(event `Recieve Nutrients_Event` :!signature `self.Recieve Nutrients`
  (params (Amount :type "Float (double-precision)"))
  ;[1 1 1] Initialise and configure Messages
  ;;[1 1 1] Recieve Nutrients from Life
  (`self.IncreaseNutrientSupplyAmount` Amount))

(event `AddLifeToMysellium_Event` :!signature `self.Add Life To Mysellium`
  (params (NewLifeToAdd :type "Actor Object Reference"))
  ;[1 1 1] Initialise and configure Messages
  ;;[1 1 1] Update Mysellium Life
  (`self.AddLifeToMysellium` NewLifeToAdd))

(event `Remove Life From Mysellium_Event` :!signature `self.Remove Life From Mysellium`
  (params (`Life To Remove` :type "Actor Object Reference"))
  ;[1 1 1] Initialise and configure Messages
  ;;[1 1 1] Update Mysellium Life
  (`self.RemoveLifeFromMysellium` `Life To Remove`))

(event `CheckLevelFailed`
  ;[1 1 1] Check if Level Failed, Show Level Failed Menu
  (if (not (> (`self.Health`) 0.0))
    (bind _asspore_2score_game_instance (cast `/Game/MyContent/Blueprints/Spore2ScoreGameInstance` (`GameplayStatics.GetGameInstance`)))
    (`/Game/MyContent/Blueprints/Spore2ScoreGameInstance.ShowLevelFailedMenu` _asspore_2score_game_instance)))

(event `IlluminateMyselliumTrail`
  ;[1 1 1] Mysellium Trail Illumination
  (for _array_element (`self.MyselliumLife`)
    (bind _asdropable_master_bp (cast `/Game/MyContent/DropableItems/DropableMaster_BP` _array_element)
      (:`then`
        (`/Game/MyContent/DropableItems/DropableMaster_BP.Illuminate` _asdropable_master_bp true))
      (:`CastFailed`
        (bind _asinteractable_master_bp (cast `/Game/MyContent/Environment/InteractableItems/InteractableMaster_BP` _array_element))
        (`/Game/MyContent/Environment/InteractableItems/InteractableMaster_BP.Illuminate` _asinteractable_master_bp true))))
  (`self.DarkenTheWorld`))

(event `DarkenTheWorld`
  ;[1 1 1] World Illumination
  (bind _returnvalue (`GameplayStatics.GetActorOfClass` "/Script/Engine.DirectionalLight"))
  (`LightComponent.SetIntensity` (`Light.LightComponent` _returnvalue) 0.0))

(event `Increasehealth`
  (params (Amount :type "Float (double-precision)"))
  ;[1 1 1] Update Health
  (set `self.Health` (`KismetMathLibrary.FClamp` (+ Amount (`self.Health`)) 0.0 (`self.MaxMysellium`))))

(event `BrightenTheWorld`
  ;[1 1 1] World Illumination
  (bind _returnvalue (`GameplayStatics.GetActorOfClass` "/Script/Engine.DirectionalLight"))
  (`LightComponent.SetIntensity` (`Light.LightComponent` _returnvalue) 10.0))

(event `Decreasehealth`
  (params (Amount :type "Float (double-precision)"))
  ;[1 1 1] Update Health
  (set `self.Health` (`KismetMathLibrary.FClamp` (- Amount (`self.Health`)) 0.0 (`self.MaxMysellium`))))

(event `UnIlluminateMySelliumTrail`
  ;[1 1 1] Mysellium Trail Illumination
  (for _array_element (`self.MyselliumLife`)
    (bind _asdropable_master_bp (cast `/Game/MyContent/DropableItems/DropableMaster_BP` _array_element)
      (:`then`
        (`/Game/MyContent/DropableItems/DropableMaster_BP.Illuminate` _asdropable_master_bp false))
      (:`CastFailed`
        (bind _asinteractable_master_bp (cast `/Game/MyContent/Environment/InteractableItems/InteractableMaster_BP` _array_element))
        (`/Game/MyContent/Environment/InteractableItems/InteractableMaster_BP.Illuminate` _asinteractable_master_bp false))))
  (`self.BrightenTheWorld`))

(event `ResetLevelValues`
  ;[1 1 1] Reset Level Properties
  (set `self.Health` 100.0)
  (set `self.Nutrients` 100.0)
  (set `self.LifeCount` 0))

(fn `AddLifeToMysellium`
  (params (NewItem :type "Actor Object Reference (by ref)"))
  (bind _asinteractable_master_bp (cast `/Game/MyContent/Environment/InteractableItems/InteractableMaster_BP` NewItem))
  (set `/Game/MyContent/Environment/InteractableItems/InteractableMaster_BP.ConnectedToMyselliumTrail` true _asinteractable_master_bp)
  (`KismetArrayLibrary.Array_AddUnique` (`self.MyselliumLife`) NewItem)
  (set `self.LifeCount` (+ (`self.LifeCount`) 1)))

(fn `CheckHealth`
  (if (< (`self.Nutrients`) 10.0)
    (set `self.Health` (`KismetMathLibrary.FClamp` (- (`self.Health`) 1.0) 0.0 100.0))))

(fn `IncreaseNutrientSupplyAmount`
  (params (NutrientAmount :type "Float (double-precision)"))
  (set `self.NutrientInput` (+ (`self.NutrientInput`) NutrientAmount))
  (set `self.Nutrients` (`KismetMathLibrary.FClamp` (+ (`self.Nutrients`) NutrientAmount) 0.0 100.0)))

(fn `PopulateMyselliumLife`)

(fn `RemoveLifeFromMysellium`
  (params (Item :type "Actor Object Reference (by ref)"))
  (cast `/Game/MyContent/Environment/InteractableItems/InteractableMaster_BP` Item)
  (`KismetArrayLibrary.Array_RemoveItem` (`self.MyselliumLife`) Item)
  (set `self.LifeCount` (- (`self.LifeCount`) 1)))

(fn `Send Nutrients to Life`
  (bind _minimalnutrientamount (`self.MinimalNutrientAmount`))
  (bind _maximum_nutrient_amount (`self.Maximum Nutrient Amount`))
  (bind _mediumnutrientamount (`self.MediumNutrientAmount`))
  (bind _maximum_nutrient_amount_2 (`self.Maximum Nutrient Amount`))
  (bind _minimalnutrientamount_2 (`self.MinimalNutrientAmount`))
  ;[1 1 1] Send Nutrients to Life
  (set `self.NutrientOutput` 0.0)
  (for _array_element (`self.MyselliumLife`)
    (bind _asnon_biological_master_bp (cast `/Game/MyContent/Environment/InteractableItems/NonBiological/NonBiologicalMaster_BP` _array_element)
      (:`then`
        (if (`/Game/MyContent/Environment/InteractableItems/NonBiological/NonBiologicalMaster_BP.IsDepleted` _asnon_biological_master_bp)
          _
          (elif (`/Game/MyContent/Environment/InteractableItems/NonBiological/NonBiologicalMaster_BP.IsSmashed` _asnon_biological_master_bp)
            (`/Game/MyContent/Environment/InteractableItems/InteractableMaster_BP.ReceiveNutrients` _asnon_biological_master_bp _minimalnutrientamount)
            (`self.UpdateNutrientLevels` _minimalnutrientamount)
            (`self.CheckHealth`)
            (else
              (`/Game/MyContent/Environment/InteractableItems/InteractableMaster_BP.ReceiveNutrients` _asnon_biological_master_bp _maximum_nutrient_amount)
              (`self.UpdateNutrientLevels` _maximum_nutrient_amount)
              (`self.CheckHealth`)))))
      (:`CastFailed`
        (bind _asbiological_master_bp (cast `/Game/MyContent/Environment/InteractableItems/Biological/BiologicalMaster_BP` _array_element))
        (bind _ishealthy (`/Game/MyContent/Environment/InteractableItems/InteractableMaster_BP.IsHealthy` _asbiological_master_bp))
        (if _ishealthy
          (bind _fullhealth (`/Game/MyContent/Environment/InteractableItems/InteractableMaster_BP.IsMaxHealth` _asbiological_master_bp))
          (if _fullhealth
            (`/Game/MyContent/Environment/InteractableItems/InteractableMaster_BP.ReceiveNutrients` _asbiological_master_bp _minimalnutrientamount_2)
            (`self.UpdateNutrientLevels` _minimalnutrientamount_2)
            (`self.CheckHealth`)
            (else
              (`/Game/MyContent/Environment/InteractableItems/InteractableMaster_BP.ReceiveNutrients` _asbiological_master_bp _mediumnutrientamount)
              (`self.UpdateNutrientLevels` _mediumnutrientamount)
              (`self.CheckHealth`)))
          (else
            (`/Game/MyContent/Environment/InteractableItems/InteractableMaster_BP.ReceiveNutrients` _asbiological_master_bp _maximum_nutrient_amount_2)
            (`self.UpdateNutrientLevels` _maximum_nutrient_amount_2)
            (`self.CheckHealth`))))))
  (set `self.NutrientInput` 0.0))

(fn `UpdateNutrientLevels`
  (params (Amount :type "Float (double-precision)"))
  (set `self.NutrientOutput` (+ (`self.NutrientOutput`) Amount))
  (set `self.Nutrients` (`KismetMathLibrary.FClamp` (- (`self.Nutrients`) Amount) 0.0 100.0)))

(fn `UserConstructionScript`)