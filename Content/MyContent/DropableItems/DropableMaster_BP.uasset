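; Base Blueprint for droppable items that link nearby vegetation and rocks to the Mysellium trail.
; BeginPlay caches the Mysellium_BP actor and starts a looping timer that polls the SphereOfInfluence for overlapping InteractableMaster_BP actors.
; Each interactable not yet connected to the trail is passed to the Mysellium to add life.
; A separate Illuminate event toggles the point light's visibility.
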(event `self.ReceiveBeginPlay`
  ;[1 1 1] Connect Vegetation and Rocks within proximity to the Mysellium Trail
  (bind _returnvalue (`GameplayStatics.GetActorOfClass` "/Game/MyContent/Mysellium/Mysellium_BP.Mysellium_BP_C"))
  (set `self.Mysellium_Ref` _returnvalue)
  (`KismetSystemLibrary.K2_SetTimerDelegate` (delegate `UpdateLifeConnected`) 1.0 true))

(event `UpdateLifeConnected`
  ;[1 1 1] Connect Vegetation and Rocks within proximity to the Mysellium Trail
  (bind _output_get (set `self.ConnectedActors` (`PrimitiveComponent.GetOverlappingActors` (`self.SphereOfInfluence`) "/Game/MyContent/InteractableItems/InteractableMaster_BP.InteractableMaster_BP_C")))
  (for _array_element _output_get
    (bind _asinteractable_master_bp (cast `/Game/MyContent/InteractableItems/InteractableMaster_BP` _array_element))
    (if (not (`/Game/MyContent/InteractableItems/InteractableMaster_BP.ConnectedToMyselliumTrail` _asinteractable_master_bp))
      (`/Game/MyContent/Mysellium/Mysellium_BP.Add Life To Mysellium` (`self.Mysellium_Ref`) _array_element))))

(event `Illuminate`
  (params (IsOn :type Boolean))
  (bind _pointlight (`self.PointLight`))
  (if IsOn
    (`SceneComponent.SetVisibility` _pointlight true false)
    (else
      (`SceneComponent.SetVisibility` _pointlight false false))))

(fn `UserConstructionScript`)