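; Mysellium Blueprint acting as a nutrient hub that feeds the life connected to its trail.
; Bound events register new interactables as connected life and add received nutrients to its clamped Health.
; A looping timer picks a supply amount from Health tiers and sends it to each registered interactable.
; Supplying never drains Health; Decreasehealth is uncalled here and subtracts in reverse, and PopulateMyselliumLife is an empty stub.
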(event `self.ReceiveBeginPlay`
  ;[1 1 1] Initialise and configure Messages
  (add `self.Add Life To Mysellium` (delegate `AddLifeToMysellium_Event`))
  (add `self.Recieve Nutrients` (delegate `Recieve Nutrients_Event`))
  ;[1 1 1] Mysellium Life Cycle
  (`KismetSystemLibrary.K2_SetTimerDelegate` (delegate `MyselliumLifeCycleTick`) 1.0 true))

(event `AddLifeToMysellium_Event` :!signature `self.Add Life To Mysellium`
  (params (NewLifeToAdd :type "Actor Object Reference"))
  (bind _asinteractable_master_bp (cast `/Game/MyContent/InteractableItems/InteractableMaster_BP` NewLifeToAdd))
  ;[1 1 1] Initialise and configure Messages
  (set `/Game/MyContent/InteractableItems/InteractableMaster_BP.ConnectedToMyselliumTrail` true _asinteractable_master_bp)
  (`KismetArrayLibrary.Array_AddUnique` (`self.MyselliumLife`) NewLifeToAdd)
  (`KismetSystemLibrary.PrintString` (`KismetSystemLibrary.GetDisplayName` NewLifeToAdd))
  (`KismetSystemLibrary.PrintString` "Life added")
  (set `self.LifeCount` (+ (`self.LifeCount`) 1)))

(event `Recieve Nutrients_Event` :!signature `self.Recieve Nutrients`
  (params (Amount :type "Float (double-precision)"))
  ;[1 1 1] Initialise and configure Messages
  (`self.Increasehealth` Amount))

(event `MyselliumLifeCycleTick`
  (bind _health (`self.Health`))
  ;[1 1 1] Mysellium Life Cycle
  ;;[1 1 1] Calculate how many nutrients can be sent to plant life
  (if (>= _health 50.0)
    (set `self.NutrientSupplyAmount` 25.0)
    ;;[1 1 1] Send Nutrient Message to Life
    (for _array_element (`self.MyselliumLife`) :!label _label
      (bind _asinteractable_master_bp (cast `/Game/MyContent/InteractableItems/InteractableMaster_BP` _array_element)
        (:`then`
          (`/Game/MyContent/InteractableItems/InteractableMaster_BP.ReceiveNutrients` _asinteractable_master_bp (`self.NutrientSupplyAmount`)))
        (:`CastFailed`
          (cast `/Game/MyContent/DropableItems/Mushroom_BP` _array_element
            (:`then`
              (`KismetSystemLibrary.PrintString` "Muashroom detcted"))
            (:`CastFailed`
              (`KismetSystemLibrary.PrintString` "Mysellium - Failed to cast to Interactable"))))))
    (elif (>= _health 25.0)
      (set `self.NutrientSupplyAmount` 15.0)
      (goto _label)
      (elif (>= _health 15.0)
        (set `self.NutrientSupplyAmount` 5.0)
        (goto _label)
        (elif (< _health 15.0)
          (set `self.NutrientSupplyAmount` 1.0)
          (goto _label))))))

(event `Increasehealth`
  (params (Amount :type "Float (double-precision)"))
  ;[1 1 1] Update Health
  (set `self.Health` (`KismetMathLibrary.FClamp` (+ Amount (`self.Health`)) 0.0 (`self.MaxMysellium`))))

(event `Decreasehealth`
  (params (Amount :type "Float (double-precision)"))
  ;[1 1 1] Update Health
  (set `self.Health` (`KismetMathLibrary.FClamp` (- Amount (`self.Health`)) 0.0 (`self.MaxMysellium`))))

(fn `GiveLife`
  (for _array_element (`self.MyselliumLife`)
    (bind _asinteractable_master_bp (cast `/Game/MyContent/InteractableItems/InteractableMaster_BP` _array_element)
      (:`then`
        (`/Game/MyContent/InteractableItems/InteractableMaster_BP.ReceiveNutrients_Event` _asinteractable_master_bp (`self.NutrientSupplyAmount`)))
      (:`CastFailed`
        (cast `/Game/MyContent/DropableItems/DropableMaster_BP` _array_element)))))

(fn `PopulateMyselliumLife`)

(fn `UserConstructionScript`)