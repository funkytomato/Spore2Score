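; Master Blueprint for non-biological interactable items that can feed nutrients to a Mysellium trail.
; HealthCycle either sends nutrients to the Mysellium reference when connected or drains clamped Health by that amount, and smashed items use a larger amount.
; Its depletion branch requires Health below zero, which the zero clamp prevents.
; Nothing in this file calls HealthCycle, and the event graph is inactive.
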(fn `Health Cycle`
  ;[1 1 1] Plant shall lose health over time, but could send it too Mysellium
  (if (`self.ConnectedToMyselliumTrail`)
    (`/Game/MyContent/Mysellium/Mysellium_BP.Recieve Nutrients` (`self.Mysellium_Ref`) (`self.NutrientAmountToSend`))
    (else
      (set `self.Health` (`KismetMathLibrary.FClamp` (- (`self.Health`) (`self.NutrientAmountToSend`)) 0.0 (`self.MaxHealth`)))))
  ;[1 1 1] If smashed, send more nutrients, if not smashed recieve more mysellium to help break down
  (if (>= (`self.Health`) 0.0)
    (if (`self.IsSmashed`)
      (set `self.NutrientAmountToSend` 5.0)
      (else
        (set `self.NutrientAmountToSend` 1.0)))
    (else
      (set `self.IsDepleted` true)
      (set `self.NutrientAmountToSend` 0.0))))

(fn `UserConstructionScript`
  (`parent.UserConstructionScript`))