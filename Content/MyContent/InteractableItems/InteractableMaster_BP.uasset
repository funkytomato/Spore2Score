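; Master Blueprint for interactable world items with health, pollution and type flags; Interact only prints clean, smash or hug messages.
; A looping timer drains health each second and flags sickness, while a bound nutrient event restores it.
; Sphere overlap by the player shows the health widget, turns the actor toward the follow camera and refreshes a light that marks low health.
; Pollution decal, sparkle and mycelium bonus helpers exist but never run here.
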(event `RotateToFacePlayer`
  (bind _defaultsceneroot (`self.DefaultSceneRoot`))
  (bind _asspore_2score_character (cast `/Game/MyContent/Characters/Blueprints/Spore2ScoreCharacter` (`GameplayStatics.GetPlayerCharacter` 0)))
  (`SceneComponent.K2_SetWorldRotation` _defaultsceneroot (`KismetMathLibrary.FindLookAtRotation` (`SceneComponent.K2_GetComponentLocation` _defaultsceneroot) (`SceneComponent.K2_GetComponentLocation` (`/Game/MyContent/Characters/Blueprints/Spore2ScoreCharacter.FollowCamera` _asspore_2score_character))) false false))

(event `IncreaseHealth`
  (params (HealthAmount :type "Float (double-precision)"))
  ;[1 1 1] Update Health Property
  (set `self.Health` (`KismetMathLibrary.FClamp` (+ HealthAmount (`self.Health`)) 0.0 (`self.MaxHealth`))))

(event `ReducePollution`
  (params (AmountToReduce :type "Float (double-precision)"))
  ;[1 1 1] Update Pollution Level
  (set `self.PollutionLevel` (- AmountToReduce (`self.PollutionLevel`))))

(event `IncreasePollution`
  (params (AmountToIncrease :type "Float (double-precision)"))
  ;[1 1 1] Update Pollution Level
  (set `self.PollutionLevel` (+ AmountToIncrease (`self.PollutionLevel`))))

(event `DecreaseHealth`
  (params (DecreaseAmount :type "Float (double-precision)"))
  ;[1 1 1] Update Health Property
  (set `self.Health` (`KismetMathLibrary.FClamp` (- DecreaseAmount (`self.Health`)) 0.0 (`self.MaxHealth`))))

(event `self.InteractionSphereOfInfluence.OnComponentBeginOverlap`
  (params (OverlappedComponent :type "PrimitiveComponent Object Reference") (OtherActor :type "Actor Object Reference") (OtherComp :type "PrimitiveComponent Object Reference") (OtherBodyIndex :type Integer) (bFromSweep :type Boolean) (SweepResult :type "HitResult Structure (by ref)"))
  ;[1 1 1] Update Plant Illumination/Sparkle corresponding plant Health
  (cast `/Game/MyContent/Characters/Blueprints/Spore2ScoreCharacter` OtherActor)
  (`self.Update Plant Health Visual`)
  (`self.RotateToFacePlayer`)
  (`SceneComponent.SetVisibility` (`self.Widget`) true false))

(event `/Game/MyContent/Interface/Score2Spore_BPI.Interact`
  ;[1 1 1] Interact with Game Items
  (`KismetSystemLibrary.PrintString` "Interacting")
  ;;[1 1 1] Cleanup Pollution
  (if (`self.Polluted`)
    (`KismetSystemLibrary.PrintString` "Clean Pollution")
    (else
      ;;[1 1 1] Is a rock, smash it, to release minerals
      (if (`self.Breakable`)
        (`KismetSystemLibrary.PrintString` "Smash Rock")
        (else
          ;;[1 1 1] Hug Tree, give some love
          (if (`self.Huggable`)
            (`KismetSystemLibrary.PrintString` "Hug!!!")))))))

(event `self.InteractionSphereOfInfluence.OnComponentEndOverlap`
  (params (OverlappedComponent :type "PrimitiveComponent Object Reference") (OtherActor :type "Actor Object Reference") (OtherComp :type "PrimitiveComponent Object Reference") (OtherBodyIndex :type Integer))
  ;[1 1 1] Update Plant Illumination/Sparkle corresponding plant Health
  (cast `/Game/MyContent/Characters/Blueprints/Spore2ScoreCharacter` OtherActor)
  (`self.Update Plant Health Visual`)
  (`SceneComponent.SetVisibility` (`self.Widget`) false false))

(event `self.ReceiveBeginPlay`
  (bind _aswidget_bp (cast `/Game/MyContent/Widgets/Widget_BP` (`WidgetComponent.GetUserWidgetObject` (`self.Widget`))))
  (bind _output_get (set `self.HealthWidget` _aswidget_bp))
  ;[1 1 1] Show the Plant's Health status on BeginPlay
  (set `/Game/MyContent/Widgets/Widget_BP.OwningActor` self _output_get)
  (`self.Update Plant Health Visual`)
  (`KismetSystemLibrary.K2_SetTimer` null "PlantHealthCycle" 1.0 true)
  ;[1 1 1] Boost Health from Mysellium
  (add `self.ReceiveNutrients` (delegate `ReceiveNutrients_Event`)))

(event `ReceiveNutrients_Event` :!signature `self.ReceiveNutrients`
  (params (Amount :type "Float (double-precision)"))
  ;[1 1 1] Boost Health from Mysellium
  (`self.IncreaseHealth` Amount))

(fn `Illuminate`
  (`SceneComponent.SetVisibility` (`self.IlluminationLight`) true false))

(fn `IsHealthy`
  (returns (IsHealthy :type Boolean))
  (return (>= (`self.Health`) (`self.LowHealthValue`))))

(fn `IsPolluted`
  (returns (IsPolluted :type Boolean))
  (bind _returnvalue (>= (`self.PollutionLevel`) (`self.HighPollutionValue`)))
  (if _returnvalue
    (set `self.Polluted` true)
    (else
      (set `self.Polluted` false)))
  (return _returnvalue))

(fn `MyselliumBonus`
  (if (`self.ConnectedToMyselliumTrail`)
    (set `self.Health` (`KismetMathLibrary.FClamp` (+ (`self.Health`) (`self.MySelliumHealthBonus`)) 0.0 100.0))))

(fn `PlantHealthCycle`
  ;[1 1 1] Plant shall lose health over time
  (bind _output_get (set `self.Health` (`KismetMathLibrary.FClamp` (- (`self.Health`) 1.0) 0.0 (`self.MaxHealth`))))
  ;[1 1 1] Set Unhealthy flag if sick
  (if (< _output_get (`self.LowHealthValue`))
    (set `self.IsUnhealthy` true)
    (else
      (set `self.IsUnhealthy` false))))

(fn `ShowPollution`
  (bind _pollutiondecal (`self.PollutionDecal`))
  (if (`self.Polluted`)
    (`SceneComponent.SetVisibility` _pollutiondecal true false)
    (else
      (`SceneComponent.SetVisibility` _pollutiondecal false false))))

(fn `Sparkle`
  (`KismetSystemLibrary.PrintString` "Make Tree Sparkle")
  (`ActorComponent.SetActive` (`self.SparkleParticles`) false false))

(fn `UnIlluminate`
  (`SceneComponent.SetVisibility` (`self.IlluminationLight`) false false))

(fn `Update Plant Health Visual`
  ;[1 1 1] Make Plant Sparkle if healthy
  (bind _ishealthy (`self.IsHealthy`))
  (if _ishealthy
    (`self.UnIlluminate`)
    (else
      (`self.Illuminate`))))

(fn `UpdateHealth`
  (set `self.Health` (- (`self.HealthLoss`) (`self.Health`)))
  (`self.MyselliumBonus`))

(fn `UserConstructionScript`)