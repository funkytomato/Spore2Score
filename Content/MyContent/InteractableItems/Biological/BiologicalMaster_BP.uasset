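; BiologicalMaster_BP is a biological interactable, evidently a plant base, that either feeds a mycelium trail or loses health over time.
; A looping timer started on BeginPlay runs Plant Health Cycle every second.
; When connected, the cycle sends nutrients to the mycelium reference; otherwise it subtracts that amount from clamped health.
; Low health flags the plant unhealthy and reduces the nutrient amount, slowing both transfer and decay.
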(event `self.ReceiveBeginPlay`
  (`parent.ReceiveBeginPlay`)
  (`KismetSystemLibrary.K2_SetTimer` null "Plant Health Cycle" 1.0 true))

(fn `Plant Health Cycle`
  ;[1 1 1] Plant shall lose health over time, but could send it too Mysellium
  (if (`self.ConnectedToMyselliumTrail`)
    (`/Game/MyContent/Mysellium/Mysellium_BP.Recieve Nutrients` (`self.Mysellium_Ref`) (`self.NutrientAmountToSend`))
    (else
      (bind _output_get (set `self.Health` (`KismetMathLibrary.FClamp` (- (`self.Health`) (`self.NutrientAmountToSend`)) 0.0 (`self.MaxHealth`))))))
  ;[1 1 1] Set Unhealthy flag if sick
  (if (< _output_get (`self.LowHealthValue`))
    (set `self.IsUnhealthy` true)
    (set `self.NutrientAmountToSend` 1.0)
    (else
      (set `self.IsUnhealthy` false)
      (set `self.NutrientAmountToSend` 5.0))))

(fn `UserConstructionScript`
  (`parent.UserConstructionScript`))